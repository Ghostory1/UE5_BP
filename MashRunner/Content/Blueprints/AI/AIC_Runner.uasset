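; AI controller for BP_Runner that fakes a player's alternating left and right inputs to power the runner.
; It caches the possessed runner, then starts a one-shot timer loop on BeginPlay with a random delay between min and max values.
; A FlipFlop alternates SimulatePowerLeft and SimulatePowerRight, re-arming the timer after each input for an irregular rhythm.
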(event Custom|SimulateInput
  (Utilities|FlowControl|FlipFlop
    (:A
      (Default|SimulatePowerLeft (Variables|Default|GetOwingRunner))
      (CallFunction|SimulateInputwithDelay))
    (:B
      (Default|SimulatePowerRight (Variables|Default|GetOwingRunner))
      (CallFunction|SimulateInputwithDelay))))

(event EventPossess
  (params (PossessedPawn :type Pawn%20Object%20Reference))
  (bind _asbp_runner (Utilities|Casting|CastToBP_Runner PossessedPawn))
  (Variables|Default|SetOwingRunner _asbp_runner))

(event EventBeginPlay
  (CallFunction|SimulateInputwithDelay))

(fn ConstructionScript)

(fn SimulateInputwithDelay
  (Utilities|Time|SetTimerbyEvent (EventDispatchers|CreateEvent :!event Custom|SimulateInput) (Math|Random|RandomFloatinRange (Variables|Default|GetMinInputDelay) (Variables|Default|GetMaxInputDelay))))